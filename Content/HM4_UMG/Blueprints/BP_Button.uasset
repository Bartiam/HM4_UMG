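; BP_Button is a proximity button that toggles the visibility of a set of world actors.
; When a Player-tagged actor enters its collision, it spawns WBP_ScreenButton, passes itself as CurrentButton and shows the cursor in Game and UI input mode.
; Leaving removes all widgets and restores game-only input.
; Its Switcher event applies IsHidden to every actor in WorldActors, then flips the flag.
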(event OnComponentBeginOverlap(Collision)
  (params (OverlappedComponent :type Primitive%20Component%20Object%20Reference) (OtherActor :type Actor%20Object%20Reference) (OtherComp :type Primitive%20Component%20Object%20Reference) (OtherBodyIndex :type Integer) (bFromSweep :type Boolean) (SweepResult :type Hit%20Result%20Structure%20%28by%20ref%29))
  (bind _returnvalue (Game|GetPlayerController 0))
  ;[1 1 1] Check overlap actor
  (if (Actor|ActorHasTag OtherActor "Player")
    ;[1 1 1] Create and add widget
    (bind _returnvalue_2 (UserInterface|CreateWidget "/Game/HM4_UMG/UI/WBP_ScreenButton.WBP_ScreenButton_C" (Game|GetPlayerController 0)))
    (UserInterface|Viewport|AddtoViewport _returnvalue_2 0)
    ;[1 1 1] Transfer current button
    (Variables|/Game/HM4_UMG/UI/WBP_ScreenButton.WBP_ScreenButton_C|SetCurrentButton _returnvalue_2 self)
    ;[1 1 1] Change input mode
    (Variables|/Script/Engine.PlayerController|SetbShowMouseCursor _returnvalue true)
    (Input|SetInputModeGameandUI _returnvalue 0 "DoNotLock" false false)))

(event OnComponentEndOverlap(Collision)
  (params (OverlappedComponent :type Primitive%20Component%20Object%20Reference) (OtherActor :type Actor%20Object%20Reference) (OtherComp :type Primitive%20Component%20Object%20Reference) (OtherBodyIndex :type Integer))
  (bind _returnvalue (Game|GetPlayerController 0))
  ;[1 1 1] Check overlap actor
  (if (Actor|ActorHasTag OtherActor "Player")
    (Viewport|RemoveAllWidgets)
    ;[1 1 1] Change input mode
    (Variables|/Script/Engine.PlayerController|SetbShowMouseCursor _returnvalue false)
    (Input|SetInputModeGameOnly _returnvalue false)))

(event EventSwitcher
  ;[1 1 1] Change objects hidden in game
  (for _array_element (Variables|Default|GetWorldActors)
    (Rendering|SetActorHiddenInGame _array_element (Variables|Default|GetbIsHidden)))
  (if (Variables|Default|GetbIsHidden)
    (Variables|Default|SetbIsHidden false)
    (else
      (Variables|Default|SetbIsHidden true))))

(fn ConstructionScript)